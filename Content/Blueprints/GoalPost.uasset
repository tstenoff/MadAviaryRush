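; Team-coloured goal post that can be displaced, eases back to its starting point, and counts scores.
; A hit on the goal restarts a five-second timer, after which Tick lerps it towards StartingPoint.
; Tick also feeds the goal's position to StartingPoint's materials for transparency and stretches a Pointer between start and goal.
; Cylinder overlaps increment Goals behind an IsOverlaping guard, and SetTeam tints the goal red or blue through a dynamic material.
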(event OnComponentBeginOverlap(Cylinder)
  (params (OverlappedComponent :type Primitive%20Component%20Object%20Reference) (OtherActor :type Actor%20Object%20Reference) (OtherComp :type Primitive%20Component%20Object%20Reference) (OtherBodyIndex :type Integer) (bFromSweep :type Boolean) (SweepResult :type Hit%20Result%20Structure%20%28by%20ref%29))
  ;[1 1 1] goal post score collision detection
  (Variables|Default|SetotherActor OtherActor)
  (if (Math|Boolean|NotEqual(Boolean) (Variables|Default|GetisOverlaping) true)
    (Math|Integer|IncrementInt (Variables|Default|Getgoals)
      (:%20%20
        (Variables|Default|SetisOverlaping true)))))

(event OnComponentEndOverlap(Cylinder)
  (params (OverlappedComponent :type Primitive%20Component%20Object%20Reference) (OtherActor :type Actor%20Object%20Reference) (OtherComp :type Primitive%20Component%20Object%20Reference) (OtherBodyIndex :type Integer))
  ;[1 1 1] goal post score collision detection
  (if (== OtherActor (Variables|Default|GetotherActor))
    (Variables|Default|SetisOverlaping false)
    (Variables|Default|SetotherActor 0)))

(event OnComponentHit(Goal)
  (params (HitComponent :type Primitive%20Component%20Object%20Reference) (OtherActor :type Actor%20Object%20Reference) (OtherComp :type Primitive%20Component%20Object%20Reference) (NormalImpulse :type Vector :default "0, 0, 0") (Hit :type Hit%20Result%20Structure%20%28by%20ref%29))
  (Variables|Default|SetpositionResetTimer 5.0)
  (Variables|Default|SetisReseting false))

(event EventBeginPlay)

(event Collision|EventActorBeginOverlap
  (params (OtherActor :type Actor%20Object%20Reference)))

(event EventTick
  (params (DeltaSeconds :type Float%20%28single-precision%29))
  (bind _goal (Variables|Default|GetGoal))
  (bind _startingpoint (Variables|Default|GetStartingPoint))
  (bind _pointer (Variables|Default|Getpointer))
  (bind _pointer_2 (Variables|Default|Getpointer))
  (bind _returnvalue (Transformation|GetWorldLocation _goal))
  (bind _returnvalue_2 (Transformation|GetWorldLocation _startingpoint))
  (Utilities|FlowControl|Sequence
    (:then_0
      ;[1 1 1] Transparency control
      (Rendering|Material|SetVectorParameterValueonMaterials (Variables|Default|GetStartingPoint) "GoalPosition" (.location (Transformation|GetWorldTransform (Variables|Default|GetGoal)))))
    (:then_1
      ;[1 1 1] Reset net position
      (bind _output_get (Variables|Default|SetpositionResetTimer (- (Variables|Default|GetpositionResetTimer) DeltaSeconds)))
      (if (<= _output_get 0.0)
        (if (not (Variables|Default|GetisReseting))
          (CallFunction|ResetTransform DeltaSeconds))))
    (:then_2
      ;[1 1 1] Rotate Arrow
      (Transformation|SetWorldTransform _pointer (Class|KismetAnimationLibrary|Lookat (Transformation|GetWorldTransform _pointer) (Transformation|GetWorldLocation (Variables|Default|GetGoal)) "0.000000, 0,1.000000" false "0, 0,1.000000" 0.0) false false)
      (Transformation|SetWorldLocation _pointer_2 (+ _returnvalue_2 (/ (- _returnvalue _returnvalue_2) 2.0)) false false)
      (Transformation|SetRelativeScale3D _pointer_2 (Math|Vector|MakeVector 0.1 0.1 (/ (Math|Vector|Distance(Vector) _returnvalue_2 _returnvalue) 1e+02))))))

(fn ConstructionScript)

(fn SetTeam
  (params (NewParam :type teamColour%20Enum :default "NewEnumerator0"))
  (bind _output_get (Variables|Default|Setteam NewParam))
  (bind _returnvalue (Rendering|Material|CreateDynamicMaterialInstance (Variables|Default|GetGoal) 0 "/Game/Materials/GoalMat.GoalMat" "None" :!class /Script/Engine.PrimitiveComponent))
  (if (Utilities|Enum|Equal(Enum) _output_get "NewEnumerator0")
    (Rendering|Material|SetVectorParameterValue _returnvalue "BaseColour" (Utilities|Struct|MakeLinearColor 1.0 0.0 0.0 0.0) :!class /Script/Engine.MaterialInstanceDynamic)
    (else
      (Rendering|Material|SetVectorParameterValue _returnvalue "BaseColour" (Utilities|Struct|MakeLinearColor 0.0 0.0 1.0 0.0) :!class /Script/Engine.MaterialInstanceDynamic))))

(fn OnRepGoals)

(fn ResetTransform
  (params (deltaTime :type Float%20%28single-precision%29))
  (bind _startingpoint (Variables|Default|GetStartingPoint))
  (bind _goal (Variables|Default|GetGoal))
  (bind _goal_2 (Variables|Default|GetGoal))
  (Transformation|SetWorldLocation _goal (Math|Vector|Lerp(Vector) (Transformation|GetWorldLocation _goal_2) (Transformation|GetWorldLocation _startingpoint) deltaTime) false true)
  (Transformation|SetRelativeRotation _goal (Math|Rotator|Lerp(Rotator) (Transformation|GetWorldRotation _goal_2) (Transformation|GetWorldRotation _startingpoint) deltaTime) false false)
  (if (<= (Math|Vector|Distance(Vector) (Transformation|GetWorldLocation (Variables|Default|GetStartingPoint)) (Transformation|GetWorldLocation (Variables|Default|GetGoal))) 0.001)
    (Variables|Default|SetisReseting false)))